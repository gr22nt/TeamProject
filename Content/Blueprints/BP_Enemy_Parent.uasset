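; BP_Enemy_Parent is a Character Blueprint, named as an enemy base class, that walks continuously forward along its control-rotation yaw.
; Tick adds that movement input, and the construction script sets walk and crouched speeds from ForwardVelocity.
; HealthCheck clears Alive and destroys the actor at zero or lower Health, but nothing in this file calls it.
; A particle emitter spawn in HealthCheck is left unconnected.
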(event EventBeginPlay)

(event Collision|EventActorBeginOverlap
  (params (OtherActor :type Actor%20Object%20Reference)))

(event EventTick
  (params (DeltaSeconds :type Float%20%28single-precision%29))
  (Pawn|Input|AddMovementInput (Math|Vector|GetForwardVector (Math|Rotator|MakeRotator 0.0 0.0 (.Yaw (Math|Rotator|BreakRotator (Pawn|GetControlRotation :!class /Script/Engine.Pawn))))) 1.0 false))

(fn ConstructionScript
  (bind _forward_velocity (Variables|Default|GetForward_Velocity))
  (bind _charactermovement (Variables|Character|GetCharacterMovement))
  (Variables|/Script/Engine.CharacterMovementComponent|SetMaxWalkSpeed _charactermovement _forward_velocity)
  (Variables|/Script/Engine.CharacterMovementComponent|SetMaxWalkSpeedCrouched _charactermovement _forward_velocity))

(fn HealthCheck
  (if (<= (Variables|Default|GetHealth) 0.0)
    (Variables|Default|SetAlive false)
    (Actor|DestroyActor)))