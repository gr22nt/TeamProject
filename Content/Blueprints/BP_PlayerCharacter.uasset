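; Player character Blueprint, apparently for a sprite-based shooter, handling movement and automatic projectile fire.
; Up and Right axes move it along control-yaw directions.
; Fire input, if alive, or ForceFiring_Now drives a Gate and Delay loop spawning projectiles from two side offsets, paired or alternating, with damage and clamped fire-rate multipliers.
; Releasing Fire closes the gate, while StopFiring_Now can also lock firing.
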(event Custom|ForceFiring_Now
  (bind _sprite (Variables|Default|GetSprite))
  (bind _returnvalue (Transformation|GetWorldLocation _sprite))
  (if (not (Variables|Default|GetLockFiring))
    (if (Variables|Default|GetCan_Fire)
      (Utilities|FlowControl|Sequence
        (:then_0
          (goto _label Open))
        (:then_1
          (Utilities|FlowControl|Gate true :!label _label
            (:Exit
              (Utilities|FlowControl|Sequence
                (:then_0
                  _)
                (:then_1
                  (Utilities|FlowControl|Delay (Math|Float|Clamp(Float) (* (Variables|Default|GetFireRate_Multi) (Variables|Default|GetFireRate)) 0.033) :!label _label_2)
                  (Variables|Default|SetCan_Fire true)
                  (goto _label)))))))
      (else
        (Utilities|FlowControl|Sequence
          (:then_0
            (goto _label Open))
          (:then_1
            (goto _label_2)))))
    (if (Variables|Default|GetFlip_Flop_Firing)
      (Utilities|FlowControl|FlipFlop
        (:A
          (Game|SpawnActorfromClass (Variables|Default|GetProjectile) (Math|Transform|MakeTransform (+ (Transformation|GetWorldLocation (Variables|Default|GetSprite)) "0.000000,100.000000,-1.000000") "0.000000,-90.000000,0.000000") "Undefined" 0 (Variables|Default|GetDamage_Multi) 3e+03 0))
        (:B
          (Game|SpawnActorfromClass (Variables|Default|GetProjectile) (Math|Transform|MakeTransform (+ (Transformation|GetWorldLocation (Variables|Default|GetSprite)) "0.000000,-100.000000,-1.000000") "0.000000,-90.000000,0.000000") "Undefined" 0 (Variables|Default|GetDamage_Multi) 3e+03 0)))
      (else
        (Game|SpawnActorfromClass (Variables|Default|GetProjectile) (Math|Transform|MakeTransform (+ _returnvalue "0.000000,100.000000,-1.000000") "0.000000,-90.000000,0.000000") "Undefined" 0 (Variables|Default|GetDamage_Multi) 3e+03 0)
        (Game|SpawnActorfromClass (Variables|Default|GetProjectile) (Math|Transform|MakeTransform (+ _returnvalue "0.000000,-100.000000,-1.000000") "0.000000,-90.000000,0.000000") "Undefined" 0 (Variables|Default|GetDamage_Multi) 3e+03 0)))
    (Variables|Default|SetCan_Fire false)))

(event Custom|StopFiring_Now
  (params (LockFiring_Input :type Boolean))
  (bind _sprite (Variables|Default|GetSprite))
  (bind _returnvalue (Transformation|GetWorldLocation _sprite))
  (if LockFiring_Input
    (Variables|Default|SetLockFiring true)
    (Utilities|FlowControl|Gate true) ; enters at Close
  ))

(event EventBeginPlay)

(event Collision|EventActorBeginOverlap
  (params (OtherActor :type Actor%20Object%20Reference)))

(event EventTick
  (params (DeltaSeconds :type Float%20%28single-precision%29)))

(event Input|ActionEvents|InputActionFire
  (params (Key :type Key%20Structure :default "None"))
  (bind _sprite (Variables|Default|GetSprite))
  (bind _returnvalue (Transformation|GetWorldLocation _sprite))
  (:Pressed
    (if (Variables|Default|GetAlive)
      (if (not (Variables|Default|GetLockFiring))
        (if (Variables|Default|GetCan_Fire)
          (Utilities|FlowControl|Sequence
            (:then_0
              (goto _label Open))
            (:then_1
              (Utilities|FlowControl|Gate true :!label _label
                (:Exit
                  (Utilities|FlowControl|Sequence
                    (:then_0
                      _)
                    (:then_1
                      (Utilities|FlowControl|Delay (Math|Float|Clamp(Float) (* (Variables|Default|GetFireRate_Multi) (Variables|Default|GetFireRate)) 0.033) :!label _label_2)
                      (Variables|Default|SetCan_Fire true)
                      (goto _label)))))))
          (else
            (Utilities|FlowControl|Sequence
              (:then_0
                (goto _label Open))
              (:then_1
                (goto _label_2)))))
        (if (Variables|Default|GetFlip_Flop_Firing)
          (Utilities|FlowControl|FlipFlop
            (:A
              (Game|SpawnActorfromClass (Variables|Default|GetProjectile) (Math|Transform|MakeTransform (+ (Transformation|GetWorldLocation (Variables|Default|GetSprite)) "0.000000,100.000000,-1.000000") "0.000000,-90.000000,0.000000") "Undefined" 0 (Variables|Default|GetDamage_Multi) 3e+03 0))
            (:B
              (Game|SpawnActorfromClass (Variables|Default|GetProjectile) (Math|Transform|MakeTransform (+ (Transformation|GetWorldLocation (Variables|Default|GetSprite)) "0.000000,-100.000000,-1.000000") "0.000000,-90.000000,0.000000") "Undefined" 0 (Variables|Default|GetDamage_Multi) 3e+03 0)))
          (else
            (Game|SpawnActorfromClass (Variables|Default|GetProjectile) (Math|Transform|MakeTransform (+ _returnvalue "0.000000,100.000000,-1.000000") "0.000000,-90.000000,0.000000") "Undefined" 0 (Variables|Default|GetDamage_Multi) 3e+03 0)
            (Game|SpawnActorfromClass (Variables|Default|GetProjectile) (Math|Transform|MakeTransform (+ _returnvalue "0.000000,-100.000000,-1.000000") "0.000000,-90.000000,0.000000") "Undefined" 0 (Variables|Default|GetDamage_Multi) 3e+03 0)))
        (Variables|Default|SetCan_Fire false))))
  (:Released
    (if (not (Variables|Default|GetLockFiring))
      (goto _label Close))))

(event Input|AxisEvents|InputAxisUp
  (params (AxisValue :type Float%20%28single-precision%29))
  (Pawn|Input|AddMovementInput (Math|Vector|GetForwardVector (Math|Rotator|MakeRotator 0.0 0.0 (.Yaw (Math|Rotator|BreakRotator (Pawn|GetControlRotation :!class /Script/Engine.Pawn))))) AxisValue false))

(event Input|AxisEvents|InputAxisRight
  (params (AxisValue :type Float%20%28single-precision%29))
  (Pawn|Input|AddMovementInput (Math|Vector|GetRightVector (Math|Rotator|MakeRotator 0.0 0.0 (.Yaw (Math|Rotator|BreakRotator (Pawn|GetControlRotation :!class /Script/Engine.Pawn))))) AxisValue false))

(fn ConstructionScript)