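; Base projectile actor that damages enemies, the player or both, depending on its HarmEnemies and HarmPlayer flags.
; The construction script sets movement speed from ProjectileSpeed, and BeginPlay rotates the actor along its velocity.
; On overlap, the other actor's first tag selects the target type, whose Health drops by Damage times DamageMulti before HealthCheck runs.
; Harmful hits destroy the projectile, even on dead targets, but living invincible players are ignored.
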(event EventBeginPlay
  (bind _returnvalue (Transformation|GetActorLocation))
  (Transformation|SetActorRotation (Math|Rotator|FindLookatRotation _returnvalue (+ _returnvalue (Transformation|GetVelocity)))))

(event Collision|EventActorBeginOverlap
  (params (OtherActor :type Actor%20Object%20Reference))
  (bind _asbp_enemy_parent (Utilities|Casting|CastToBP_Enemy_Parent OtherActor))
  (bind _asbp_player_character (Utilities|Casting|CastToBP_PlayerCharacter OtherActor))
  (switch name (Utilities|Array|Get(acopy) (Variables|/Script/Engine.Actor|GetTags OtherActor))
    (:Enemy
      (if (Variables|Default|GetHarm_Enemies)
        (if (> (Variables|/Game/Blueprints/BP_Enemy_Parent.BP_Enemy_Parent_C|GetHealth _asbp_enemy_parent) 0.0)
          (Variables|/Game/Blueprints/BP_Enemy_Parent.BP_Enemy_Parent_C|SetHealth _asbp_enemy_parent (- (Variables|/Game/Blueprints/BP_Enemy_Parent.BP_Enemy_Parent_C|GetHealth _asbp_enemy_parent) (* (Variables|Default|GetDamage) (Variables|Default|GetDamage_Multi))))
          (Default|HealthCheck _asbp_enemy_parent))
        (Actor|DestroyActor)))
    (:Player
      (if (Variables|Default|GetHarm_Player)
        (if (Variables|/Game/Blueprints/BP_PlayerCharacter.BP_PlayerCharacter_C|GetAlive _asbp_player_character)
          (if (not (Variables|/Game/Blueprints/BP_PlayerCharacter.BP_PlayerCharacter_C|GetInvincible _asbp_player_character))
            (Variables|/Game/Blueprints/BP_PlayerCharacter.BP_PlayerCharacter_C|SetHealth _asbp_player_character (- (Variables|/Game/Blueprints/BP_PlayerCharacter.BP_PlayerCharacter_C|GetHealth _asbp_player_character) (* (Variables|Default|GetDamage_Multi) (Variables|Default|GetDamage))))
            (Default|HealthCheck _asbp_player_character)
            (Actor|DestroyActor :!label _label))
          (else
            (goto _label)))))))

(event EventTick
  (params (DeltaSeconds :type Float%20%28single-precision%29)))

(fn ConstructionScript
  (bind _projectilemovement (Variables|Default|GetProjectileMovement))
  (bind _projectile_speed (Variables|Default|GetProjectile_Speed))
  (Variables|/Script/Engine.ProjectileMovementComponent|SetInitialSpeed _projectilemovement _projectile_speed)
  (Variables|/Script/Engine.ProjectileMovementComponent|SetMaxSpeed _projectilemovement _projectile_speed))